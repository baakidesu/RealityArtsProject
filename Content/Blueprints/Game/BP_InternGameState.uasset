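; Game state Blueprint that runs the match countdown and tracks the current wave number.
; A looping one-second timer starts on BeginPlay and, after a one-second delay, decrements the minute and second counters until both reach zero.
; Each minute rollover advances the wave, and every tick broadcasts time and wave through an event dispatcher for the UI.
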(event `self.ReceiveBeginPlay`
  (`KismetSystemLibrary.K2_SetTimerDelegate` (delegate `Timer`) 1.0 true))

(event `Timer`
  ; Check if game ended
  (if (not (`self.CheckIsTimeEnded`))
    (`KismetSystemLibrary.Delay` 1.0)
    (if (> 1 (`self.Second`))
      (set `self.Second` 59)
      (`/Engine/EditorBlueprintResources/StandardMacros.DecrementInt` (`self.Minute`)
        (:`  `
          (`/Engine/EditorBlueprintResources/StandardMacros.IncrementInt` (`self.OnWhichWave`)
            (:`  `
              (`self.DP_UpdateTimeAndWaveOnUI` (`self.Second`) (`self.Minute`) (`self.OnWhichWave`))))))
      (else
        (`/Engine/EditorBlueprintResources/StandardMacros.DecrementInt` (`self.Second`)
          (:`  `
            (`self.DP_UpdateTimeAndWaveOnUI` (`self.Second`) (`self.Minute`) (`self.OnWhichWave`))))))))

(fn `CheckIsTimeEnded`
  (returns (ReturnValue :type Boolean))
  (return (and (== (`self.Minute`) 0) (== (`self.Second`) 0))))

(fn `UserConstructionScript`)