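; Game mode that runs the match countdown clock and drives enemy wave progression.
; A looping one-second timer checks for zero time to send the game-end message to the player HUD, otherwise ticks the clock after a Delay.
; Each minute rollover calls C++ to advance the wave and spawn enemies, and every tick broadcasts time and wave to the UI through a dispatcher.
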(event `self.ReceiveBeginPlay`
  (`KismetSystemLibrary.K2_SetTimerDelegate` (delegate `Timer`) 1.0 true))

(event `Timer`
  ; Check if game ended
  (if (`self.CheckIsTimeEnded`)
    (message `/Game/Blueprints/Interfaces/BPI_CombatInterface.GameShouldEnd` (`self.GetPlayerHUD`) true)
    (else
      ;[0.004182 0.15 0 0.5] Timer Logic Here, Increasing Wave by Killing Enemies logic implemented in C++
      (`KismetSystemLibrary.Delay` 1.0)
      (if (> 1 (`self.Second`))
        (set `self.Second` 59)
        (`/Engine/EditorBlueprintResources/StandardMacros.DecrementInt` (`self.Minute`)
          (:`  `
            ;;[0.15 0.04825 0 0.5] C++ implemented function
            (`self.IncreaseWaveIndexAndSpawnEnemies`)
            (`self.DP_UpdateTimeAndWaveOnUI` (`self.Second`) (`self.Minute`) (`self.CurrentWaveIndex`))))
        (else
          (`/Engine/EditorBlueprintResources/StandardMacros.DecrementInt` (`self.Second`)
            (:`  `
              (`self.DP_UpdateTimeAndWaveOnUI` (`self.Second`) (`self.Minute`) (`self.CurrentWaveIndex`)))))))))

(fn `CheckIsTimeEnded`
  (returns (ReturnValue :type Boolean))
  (return (and (== (`self.Second`) 0) (== (`self.Minute`) 0))))

(fn `GetPlayerHUD`
  (returns (ReturnValue :type "HUD Object Reference"))
  (return (`PlayerController.GetHUD` (`GameplayStatics.GetPlayerController` 0))))

(fn `UserConstructionScript`)