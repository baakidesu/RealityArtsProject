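; Enemy gameplay ability for a swordsman's melee slash that damages players in front of the attacker.
; It plays the attack montage and waits for the weapon gameplay event, then runs a forward multi-sphere trace with debug drawing.
; Each Player-tagged actor not already recorded as hit receives GE_SwordSlash.
; The ability ends after the hit or montage end; a blackboard-bool helper is defined but never called.
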(event `self.K2_ActivateAbility`
  (`AbilityTask_PlayMontageAndWait.CreatePlayMontageAndWaitProxy` "None" "/Game/Animations/Swordman/AM_Swordsman_Attack.AM_Swordsman_Attack"
    (:`then`
      (`AbilityTask_WaitGameplayEvent.WaitGameplayEvent` (struct :`TagName` "Abilities.Attack.Weapon") null
        (:`EventReceived`
          (bind _outhits (`self.GetLivePlayers`))
          (`self.HitPlayers` _outhits)
          (`self.K2_EndAbility`))))
    (:`OnCompleted`
      (`self.K2_EndAbility` :!label _label))
    (:`OnInterrupted`
      (goto _label))
    (:`OnCancelled`
      (goto _label))))

(event `self.K2_OnEndAbility`
  (params (bWasCancelled :type Boolean)))

(fn `GetLivePlayers`
  (returns (OutHits :type "Array of HitResult Structure"))
  (locals (Start :type "Vector Structure" :default (0.0 0.0 0.0)) (End :type "Vector Structure"))
  (set `local.Start` (`Actor.K2_GetActorLocation` (`self.GetAvatarActorFromActorInfo`)))
  (set `local.End` (+ (* (`Actor.GetActorForwardVector` (`self.GetAvatarActorFromActorInfo`)) 300) (`local.Start`)))
  (bind _outhits (`KismetSystemLibrary.SphereTraceMulti` :`Start` (`local.Start`) :`End` (`local.End`) :`Radius` 80.0 :`TraceChannel` "TraceTypeQuery1" :`DrawDebugType` "ForDuration"))
  (return _outhits))

(fn `HitPlayers`
  (params (Array :type "Array of HitResult Structure"))
  (for _array_element Array
    (bind (_bblockinghit _binitialoverlap _time _distance _location _impactpoint _normal _impactnormal _physmat _hitactor) (`GameplayStatics.BreakHitResult` _array_element))
    (if (`self.IsCorrectPlayerToHit` _hitactor)
      (`KismetArrayLibrary.Array_Add` (`self.ActorGotHit`) _hitactor)
      (`AbilitySystemComponent.BP_ApplyGameplayEffectToSelf` :`self` (`AbilitySystemBlueprintLibrary.GetAbilitySystemComponent` _hitactor) :`GameplayEffectClass` "/Game/Blueprints/AbilitySystem/GameplayEffects/GE_SwordSlash.GE_SwordSlash_C" :`Level` 1.0)))
  (return))

(fn `IsCorrectPlayerToHit`
  (params (HitActor :type "Actor Object Reference (by ref)"))
  (returns (ReturnValue :type Boolean))
  (return (and (`Actor.ActorHasTag` HitActor "Player") (== (`KismetArrayLibrary.Array_Find` (`self.ActorGotHit`) HitActor) -1))))

(fn `SetBlackboardBool`
  (params (DidHit :type Boolean))
  (bind _blackboard (`AIController.Blackboard` (`AIBlueprintHelperLibrary.GetAIController` (`self.GetAvatarActorFromActorInfo`)))
    (:`then`
      (`BlackboardComponent.SetValueAsBool` _blackboard (`self.BoolKeyName`) DidHit)
      (return))
    (:`else`)))