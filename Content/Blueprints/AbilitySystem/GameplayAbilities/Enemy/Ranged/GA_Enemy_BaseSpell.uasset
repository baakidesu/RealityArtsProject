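; Gameplay ability for the base spell of a ranged enemy, which plays the witch attack montage.
; On activation it sends the avatar the player pawn's location as a facing target, then starts the montage with root motion translation scaled to zero.
; It ends on the base spell gameplay event or when the montage completes, is interrupted or is cancelled.
; The graph itself spawns no projectile and applies no damage.
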(event `self.K2_ActivateAbility`
  (message `/Game/Blueprints/Interaction/BPI_Combat.UpdateFacingTarget` (`self.GetAvatarActorFromActorInfo`) (`Actor.K2_GetActorLocation` (`GameplayStatics.GetPlayerPawn` 0)))
  (`AbilityTask_PlayMontageAndWait.CreatePlayMontageAndWaitProxy` "None" "/Game/Characters/Animations/Witch/AM_Witch_Attack.AM_Witch_Attack" 1.0 "None" true 0.0
    (:`then`
      (`AbilityTask_WaitGameplayEvent.WaitGameplayEvent` (struct :`TagName` "Abilities.Attack.Enemy.Ranged.BaseSpell") null
        (:`EventReceived`
          (`self.K2_EndAbility`))))
    (:`OnCompleted`
      (`self.K2_EndAbility` :!label _label))
    (:`OnInterrupted`
      (goto _label))
    (:`OnCancelled`
      (goto _label))))