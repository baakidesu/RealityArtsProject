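; Gameplay ability that lets an AI-controlled avatar hit the player, BP_Ygritte.
; On activation it sets a Blackboard bool, reads the target from the Blackboard and has that target's Ability System Component apply GE_BasicHit to itself.
; It ends after a short delay, clearing the bool in OnEndAbility.
; A failed cast stops execution before EndAbility, leaving the bool set.
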(event `self.K2_ActivateAbility`
  (`self.SetBlackboardBool` true)
  (bind _asbp_ygritte (cast `/Game/Blueprints/Characters/Ygritte/BP_Ygritte` (`BlackboardComponent.GetValueAsObject` (`AIController.Blackboard` (`AIBlueprintHelperLibrary.GetAIController` (`self.GetAvatarActorFromActorInfo`))) (`self.TargetPlayer`))))
  (bind _returnvalue (`AbilitySystemComponent.BP_ApplyGameplayEffectToSelf` :`self` (`AbilitySystemBlueprintLibrary.GetAbilitySystemComponent` _asbp_ygritte) :`GameplayEffectClass` "/Game/Blueprints/AbilitySystem/GameplayEffects/GE_BasicHit.GE_BasicHit_C" :`Level` 1.0))
  (set `self.ActiveGameplayEffect` _returnvalue)
  (`KismetSystemLibrary.Delay` 3.0)
  (`self.K2_EndAbility`))

(event `self.K2_OnEndAbility`
  (params (bWasCancelled :type Boolean))
  (`self.SetBlackboardBool` false))

(fn `SetBlackboardBool`
  (params (DidHit :type Boolean))
  (bind _blackboard (`AIController.Blackboard` (`AIBlueprintHelperLibrary.GetAIController` (`self.GetAvatarActorFromActorInfo`)))
    (:`then`
      (`BlackboardComponent.SetValueAsBool` _blackboard (`self.BoolKeyName`) DidHit)
      (return))
    (:`else`)))