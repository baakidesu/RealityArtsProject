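; Player punch gameplay ability that plays a punch montage and damages enemies in front of the avatar.
; A montage gameplay event triggers a short forward sphere trace, applying GE_SwordSlash and a punch sound to Enemy-tagged actors not already in ActorGotHit.
; The ability ends when the montage completes or is interrupted or cancelled, or after a delay following the hit.
; A blackboard helper is defined but never called.
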(event `self.K2_ActivateAbility`
  (`AbilityTask_PlayMontageAndWait.CreatePlayMontageAndWaitProxy` "None" "/Game/Characters/Animations/Player/AM_Player_Punch.AM_Player_Punch"
    (:`then`
      (`AbilityTask_WaitGameplayEvent.WaitGameplayEvent` (struct :`TagName` "Abilities.Attack.Player.Punch") null
        (:`EventReceived`
          (bind _outhits (`self.GetLivePlayers`))
          (`self.HitPlayers` _outhits)
          (`KismetSystemLibrary.Delay` 3.0)
          (`self.K2_EndAbility`))))
    (:`OnCompleted`
      (`self.K2_EndAbility` :!label _label))
    (:`OnInterrupted`
      (goto _label))
    (:`OnCancelled`
      (goto _label))))

(event `self.K2_OnEndAbility`
  (params (bWasCancelled :type Boolean)))

(fn `GetLivePlayers`
  (returns (OutHits :type "Array of HitResult Structure"))
  (locals (Start :type "Vector Structure" :default (0.0 0.0 0.0)) (End :type "Vector Structure"))
  (set `local.Start` (`Actor.K2_GetActorLocation` (`self.GetAvatarActorFromActorInfo`)))
  (set `local.End` (+ (* (`Actor.GetActorForwardVector` (`self.GetAvatarActorFromActorInfo`)) 200) (`local.Start`)))
  (bind _outhits (`KismetSystemLibrary.SphereTraceMulti` (`local.Start`) (`local.End`) 40.0 "TraceTypeQuery1"))
  (return _outhits))

(fn `HitPlayers`
  (params (Array :type "Array of HitResult Structure"))
  (for _array_element Array
    (bind (_bblockinghit _binitialoverlap _time _distance _location _impactpoint _normal _impactnormal _physmat _hitactor) (`GameplayStatics.BreakHitResult` _array_element))
    (if (`self.IsCorrectPlayerToHit` _hitactor)
      (`KismetArrayLibrary.Array_Add` (`self.ActorGotHit`) _hitactor)
      (`AbilitySystemComponent.BP_ApplyGameplayEffectToSelf` :`self` (`AbilitySystemBlueprintLibrary.GetAbilitySystemComponent` _hitactor) :`GameplayEffectClass` "/Game/Blueprints/AbilitySystem/GameplayEffects/Enemy/GE_SwordSlash.GE_SwordSlash_C" :`Level` 1.0)
      (`GameplayStatics.PlaySoundAtLocation` "/Game/SFX/Punch/SC_Punch.SC_Punch" _location (struct) 1.0 1.0 0.0 null null null null)))
  (return))

(fn `IsCorrectPlayerToHit`
  (params (HitActor :type "Actor Object Reference (by ref)"))
  (returns (ReturnValue :type Boolean))
  (return (and (`Actor.ActorHasTag` HitActor "Enemy") (== (`KismetArrayLibrary.Array_Find` (`self.ActorGotHit`) HitActor) -1))))

(fn `SetBlackboardBool`
  (params (DidHit :type Boolean))
  (bind _blackboard (`AIController.Blackboard` (`AIBlueprintHelperLibrary.GetAIController` (`self.GetAvatarActorFromActorInfo`)))
    (:`then`
      (`BlackboardComponent.SetValueAsBool` _blackboard (`self.BoolKeyName`) DidHit)
      (return))
    (:`else`)))