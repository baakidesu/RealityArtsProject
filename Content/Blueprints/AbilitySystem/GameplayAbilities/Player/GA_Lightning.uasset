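; Player lightning gameplay ability that zaps and stuns nearby enemies.
; Plays a lightning montage and waits for its gameplay event, then runs a stationary multi-sphere trace around the avatar via GetLivePlayers, with debug drawing on.
; Enemy-tagged hits get a red zap Niagara effect and a StunMessage call.
; The ability ends after a delay, or when the montage completes, is interrupted or is cancelled.
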(event `self.K2_ActivateAbility`
  (`AbilityTask_PlayMontageAndWait.CreatePlayMontageAndWaitProxy` "None" "/Game/Characters/Animations/Player/AM_Player_Lightning.AM_Player_Lightning"
    (:`then`
      (`AbilityTask_WaitGameplayEvent.WaitGameplayEvent` (struct :`TagName` "Abilities.Attack.Player.Lightning") null
        (:`EventReceived`
          (bind _outhits (`self.GetLivePlayers`))
          (for _array_element _outhits
            (bind (_bblockinghit _binitialoverlap _time _distance _location _impactpoint _normal _impactnormal _physmat _hitactor) (`GameplayStatics.BreakHitResult` _array_element))
            (if (`Actor.ActorHasTag` _hitactor "Enemy")
              (`NiagaraFunctionLibrary.SpawnSystemAtLocation` "/Game/VFX/Vefects/Zap_VFX/VFX/Zap/Particles/NS_Zap_01_Red.NS_Zap_01_Red" _impactpoint)
              (message `/Game/Blueprints/Interaction/BPI_Combat.Stun` _hitactor)))
          (`KismetSystemLibrary.Delay` 5.0)
          (`self.K2_EndAbility`))))
    (:`OnCompleted`
      (`self.K2_EndAbility` :!label _label))
    (:`OnInterrupted`
      (goto _label))
    (:`OnCancelled`
      (goto _label))))

(fn `GetLivePlayers`
  (returns (OutHits :type "Array of HitResult Structure"))
  (bind _returnvalue (`Actor.K2_GetActorLocation` (`self.GetAvatarActorFromActorInfo`)))
  (bind _outhits (`KismetSystemLibrary.SphereTraceMulti` :`Start` _returnvalue :`End` _returnvalue :`Radius` 600.0 :`TraceChannel` "TraceTypeQuery1" :`DrawDebugType` "ForDuration"))
  (return _outhits))