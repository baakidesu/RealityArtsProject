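; Player controller that runs the upgrade menu and applies chosen upgrades to the player pawn through GAS.
; A debug key on C opens the upgrade widget in UI-only input with the cursor shown.
; UpgradeEffect closes the widget, restores game input and passes the chosen tag and effect to UpgradeGameplayAbility.
; That function adds a non-replicated loose tag, using its count as the applied effect's level so repeated picks scale.
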(event EventBeginPlay
  (Variables|Default|SetASC (Ability|GetAbilitySystemComponent (Game|Player|GetPlayerPawn 0)))
  (Variables|Default|SetPlayerPawn (Game|Player|GetPlayerPawn 0)))

(event EventUpgradeEffect
  (params (GameplayEffectClass :type Gameplay%20Effect%20Class%20Reference) (GameplayTag :type Gameplay%20Tag%20Structure))
  (bind _upgradewidget (Variables|Default|GetUpgradeWidget)
    (:then
      (Widget|RemovefromParent _upgradewidget)
      (CallFunction|UpgradeGameplayAbility GameplayTag GameplayEffectClass)
      (Variables|Default|SetbShowMouseCursor false)
      (Input|SetInputModeGameOnly self false))
    (:else)))

(event Input|KeyboardEvents|DebugKeyC
  (params (Key :type Key%20Structure :default "None") (ActionValue :type Input%20Action%20Value%20Structure))
  (:Pressed
    (bind _returnvalue (UserInterface|CreateWidget "/Game/Blueprints/Widget/Upgrades/WBP_UpgradeWidget.WBP_UpgradeWidget_C" self))
    (bind _output_get (Variables|Default|SetUpgradeWidget _returnvalue))
    (UserInterface|Viewport|AddtoViewport _output_get 0)
    (Variables|Default|SetbShowMouseCursor true)
    (Input|SetInputModeUIOnly self (Variables|Default|GetUpgradeWidget) "DoNotLock" false)))

(fn ConstructionScript)

(fn CreateConditionWidget)

(fn UpgradeGameplayAbility
  (params (Gameplay%20Tag :type Gameplay%20Tag%20Structure) (GameplayEffectClass :type Gameplay%20Effect%20Class%20Reference))
  (Ability|GameplayEffect|AddLooseGameplayTags (Variables|Default|GetPlayerPawn) (GameplayTags|MakeGameplayTagContainerfromArray (Utilities|Array|MakeArray Gameplay%20Tag)))
  (bind _asc (Variables|Default|GetASC)
    (:then
      (GameplayEffects|ApplyGameplayEffectToSelf :self _asc :GameplayEffectClass GameplayEffectClass :Level (Math|Conversions|ToFloat(Integer) (Class|AbilitySystemComponent|GetGameplayTagCount (Variables|Default|GetASC) Gameplay%20Tag))))
    (:else)))