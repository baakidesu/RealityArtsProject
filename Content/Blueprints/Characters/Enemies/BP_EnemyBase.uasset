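; Base enemy Blueprint built on the Gameplay Ability System, with a health bar widget.
; On BeginPlay it grants the enemy's gameplay ability, applies its gameplay effect to itself and assigns itself as the health bar widget's owner.
; ActivateHitEnemyAbility checks that the other actor is valid and tagged Player, then tries to activate the hard-coded GA_SwordSlash ability rather than the configurable granted one.
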(event `self.ReceiveBeginPlay`
  (`parent.ReceiveBeginPlay`)
  (`self.InitializeAttributeSetAndGiveBaseAbility`)
  (`self.SetWidget`))

(fn `ActivateHitEnemyAbility`
  (params (OtherActor :type "Actor Object Reference"))
  (`/Engine/EditorBlueprintResources/StandardMacros.IsValid` OtherActor
    (:`Is Valid`
      (if (`self.ActorHasTag` OtherActor "Player")
        (`AbilitySystemComponent.TryActivateAbilityByClass` (`self.AbilitySystemComponent`) "/Game/Blueprints/AbilitySystem/GameplayAbilities/Enemy/Melee/GA_SwordSlash.GA_SwordSlash_C" true)))))

(fn `InitializeAttributeSetAndGiveBaseAbility`
  (`AbilitySystemComponent.K2_GiveAbility` (`self.AbilitySystemComponent`) (`self.EnemyGameplayAbility`) 1 -1)
  (`AbilitySystemComponent.BP_ApplyGameplayEffectToSelf` :`self` (`self.AbilitySystemComponent`) :`GameplayEffectClass` (`self.EnemyGameplayEffect`)))

(fn `SetWidget`
  (bind _aswbp_progress_bar_en (cast `/Game/Blueprints/Widget/ProgressBar/Enemy/WBP_ProgressBarEn` (`WidgetComponent.GetWidget` (`self.HealthBarWidget`))))
  (set `/Game/Blueprints/Widget/ProgressBar/Enemy/WBP_ProgressBarEn.OwnerPlayer` self _aswbp_progress_bar_en))

(fn `UserConstructionScript`)