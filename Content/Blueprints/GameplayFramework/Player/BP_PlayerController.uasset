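; Player controller that applies upgrades to the player pawn through the Gameplay Ability System.
; BeginPlay caches the pawn and its ability system component.
; UpgradeEffect adds a non-replicated loose gameplay tag, applies the given effect, if valid, with that tag's count as its level, then unfocuses the upgrade widget.
; The tag count thus acts as a stacking upgrade level; CreateConditionWidget is an empty stub.
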(event `self.ReceiveBeginPlay`
  (set `self.ASC` (`AbilitySystemBlueprintLibrary.GetAbilitySystemComponent` (`GameplayStatics.GetPlayerPawn` 0)))
  (set `self.PlayerPawn` (`GameplayStatics.GetPlayerPawn` 0)))

(event `/Game/Blueprints/Interaction/BPI_Widget.UpgradeEffect`
  (params (GameplayEffectClass :type "GameplayEffect Class Reference") (GameplayTag :type "GameplayTag Structure"))
  (`self.UpgradeGameplayAbility` GameplayEffectClass GameplayTag)
  (`self.UnfocusUpgradeWidget`))

(fn `CreateConditionWidget`)

(fn `UpgradeGameplayAbility`
  (params (GameplayEffectClass :type "GameplayEffect Class Reference") (`Gameplay Tag` :type "GameplayTag Structure"))
  (`AbilitySystemBlueprintLibrary.AddLooseGameplayTags` (`self.PlayerPawn`) (`BlueprintGameplayTagLibrary.MakeGameplayTagContainerFromArray` (`|MakeArray` `Gameplay Tag`)))
  (if (`KismetSystemLibrary.IsValidClass` GameplayEffectClass)
    (`AbilitySystemComponent.BP_ApplyGameplayEffectToSelf` :`self` (`self.ASC`) :`GameplayEffectClass` GameplayEffectClass :`Level` (`KismetMathLibrary.Conv_IntToDouble` (`AbilitySystemComponent.GetGameplayTagCount` (`self.ASC`) `Gameplay Tag`)))))

(fn `UserConstructionScript`)