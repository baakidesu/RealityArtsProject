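; Spell projectile actor that applies GE_Projectile through the Gameplay Ability System to the first valid "Enemy"-tagged actor it hits.
; On sphere overlap it removes its trail and movement components, plays success or fail sound and Niagara effects, then destroys itself after a short delay.
; The effect level comes from the player's Upgrades.Projectile tag count, and CanThisOrbHit prevents repeat hits.
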(event `self.ReceiveBeginPlay`)

(event `self.Sphere.OnComponentBeginOverlap`
  (params (OverlappedComponent :type "PrimitiveComponent Object Reference") (OtherActor :type "Actor Object Reference") (OtherComp :type "PrimitiveComponent Object Reference") (OtherBodyIndex :type Integer) (bFromSweep :type Boolean) (SweepResult :type "HitResult Structure (by ref)"))
  (`self.DeleteTrace`)
  (if (`self.CanHit` OtherActor)
    (`self.HandleSucsessfullHit` OtherActor)
    (else
      (`self.PlaySoundEffect` false)
      (`self.PlayHitEffect`)))
  (`self.DestroyProjectile`))

(event `DestroyProjectile`
  (`KismetSystemLibrary.Delay` 1.0)
  (`self.K2_DestroyActor`))

(fn `CanHit`
  (params (OtherActor :type "Actor Object Reference"))
  (returns (ReturnValue :type Boolean))
  (return (and (`self.ActorHasTag` OtherActor "Enemy") (`KismetSystemLibrary.DoesImplementInterface` OtherActor "/Script/GameplayAbilities.AbilitySystemInterface") (`self.CanThisOrbHit`))))

(fn `DeleteTrace`
  (bind _projectiletraceniagara (`self.ProjectileTraceNiagara`)
    (:`then`
      (`ActorComponent.K2_DestroyComponent` _projectiletraceniagara)
      (bind _projectilemovement (`self.ProjectileMovement`)
        (:`then`
          (`ActorComponent.K2_DestroyComponent` _projectilemovement))
        (:`else`
          _))
      (return))
    (:`else`)))

(fn `HandleSucsessfullHit`
  (params (Actor :type "Actor Object Reference"))
  (`|ExecutionSequence`
    (:`then_0`
      (set `self.CanThisOrbHit` false)
      (`AbilitySystemComponent.BP_ApplyGameplayEffectToSelf` :`self` (`AbilitySystemBlueprintLibrary.GetAbilitySystemComponent` Actor) :`GameplayEffectClass` "/Game/Blueprints/AbilitySystem/GameplayEffects/Projectile/GE_Projectile.GE_Projectile_C" :`Level` (`KismetMathLibrary.Conv_IntToDouble` (`AbilitySystemComponent.GetGameplayTagCount` (`AbilitySystemBlueprintLibrary.GetAbilitySystemComponent` (`GameplayStatics.GetPlayerPawn` 0)) (struct :`TagName` "Upgrades.Projectile")))))
    (:`then_1`
      (`NiagaraFunctionLibrary.SpawnSystemAtLocation` "/Game/MixedVFX/Particles/Projectiles/Hits/NS_VampireArrow_Hit.NS_VampireArrow_Hit" (`SceneComponent.K2_GetComponentLocation` (`self.Sphere`)) (struct) (3.0 3.0 3.0)))
    (:`then_2`
      (`self.PlaySoundEffect` true))))

(fn `PlayHitEffect`
  (bind _returnvalue (`NiagaraFunctionLibrary.SpawnSystemAttached` "/Game/MixedVFX/Particles/Projectiles/Hits/NS_Projectile_01_Hit.NS_Projectile_01_Hit" (`self.Sphere`) "None" (0.0 0.0 0.0) (struct) "KeepRelativeOffset"))
  (set `self.ProjectileHitNiagara` _returnvalue)
  (return))

(fn `PlaySoundEffect`
  (params (IsSuccessful :type Boolean))
  (bind _returnvalue (`SceneComponent.K2_GetComponentLocation` (`self.Sphere`)))
  (if IsSuccessful
    (`GameplayStatics.PlaySoundAtLocation` "/Game/SFX/Projectile/SC_ProjectileSuccessfulHit.SC_ProjectileSuccessfulHit" _returnvalue (struct) 1.0 1.0 0.0 null null null null)
    (else
      (`GameplayStatics.PlaySoundAtLocation` "/Game/SFX/Projectile/SC_ProjectileFailHit.SC_ProjectileFailHit" _returnvalue (struct) 1.0 1.0 0.0 null null null null))))

(fn `UserConstructionScript`)