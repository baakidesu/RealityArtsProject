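; BP_InternProjectile is a spell projectile that applies a Gameplay Ability System effect to actors it hits.
; On sphere overlap it calls BeginOverlap and the hit handler, then destroys itself after a one-second delay.
; For ability-system targets, the handler applies GE_Projectile at a level equal to the player's Upgrades.Projectile tag count and spawns hit Niagara.
; Any handled overlap clears CanThisOrbHit, which this graph never checks.
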(event `self.SphereComponent.OnComponentBeginOverlap`
  (params (OverlappedComponent :type "PrimitiveComponent Object Reference") (OtherActor :type "Actor Object Reference") (OtherComp :type "PrimitiveComponent Object Reference") (OtherBodyIndex :type Integer) (bFromSweep :type Boolean) (SweepResult :type "HitResult Structure (by ref)"))
  (`self.BeginOverlap` OtherActor)
  (`self.HandleSucsessfullHit` OtherActor)
  (`self.DestroyProjectile`))

(event `DestroyProjectile`
  (`KismetSystemLibrary.Delay` 1.0)
  (`self.K2_DestroyActor`))

(fn `HandleSucsessfullHit`
  (params (Actor :type "Actor Object Reference"))
  (if (`KismetSystemLibrary.DoesImplementInterface` Actor "/Script/GameplayAbilities.AbilitySystemInterface")
    (set `self.CanThisOrbHit` false)
    (`|ExecutionSequence`
      (:`then_0`
        (`AbilitySystemComponent.BP_ApplyGameplayEffectToSelf` :`self` (`AbilitySystemBlueprintLibrary.GetAbilitySystemComponent` Actor) :`GameplayEffectClass` "/Game/Blueprints/AbilitySystem/GameplayEffects/Projectile/GE_Projectile.GE_Projectile_C" :`Level` (`KismetMathLibrary.Conv_IntToDouble` (`AbilitySystemComponent.GetGameplayTagCount` (`AbilitySystemBlueprintLibrary.GetAbilitySystemComponent` (`GameplayStatics.GetPlayerPawn` 0)) (struct :`TagName` "Upgrades.Projectile"))))
        (set `self.SuccessfulHit` true))
      (:`then_1`
        (`NiagaraFunctionLibrary.SpawnSystemAtLocation` (`self.SuccessfulHitNiagaraEffect`) (`self.K2_GetActorLocation`) (struct) (3.0 3.0 3.0))))
    (else
      (set `self.CanThisOrbHit` false)
      (return))))

(fn `UserConstructionScript`)